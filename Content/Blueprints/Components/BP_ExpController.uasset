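; Experience controller component that tracks current Exp, required Exp and level, losing Exp on player death.
; Gain and loss events adjust Exp, clamping losses at zero, and broadcast the change.
; When Exp reaches the requirement, it requests the next level.
; UpdateRequiredExp stores the new level and requirement, subtracts that passed requirement from Exp, then re-checks, allowing chained level-ups.
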(event `OnExpLost`
  (params (val :type "Float (double-precision)"))
  ; Clamp 0
  (bind _output_get (set `self.Exp` (`KismetMathLibrary.FClamp` (- (`self.Exp`) val) 0.0 (`self.Exp`))))
  (`self.OnExpChanged` _output_get (`self.RequiredExp`)))

(event `OnExpGained`
  (params (value :type "Float (double-precision)"))
  ; 계산.
  (bind _output_get (set `self.Exp` (+ (`self.Exp`) value)))
  (`self.OnExpChanged` _output_get (`self.RequiredExp`))
  ; CanLevelUp
  (if (>= (`self.Exp`) (`self.RequiredExp`))
    (`self.OnLevelUpRequested` (+ (`self.CurrentLevel`) 1))))

(event `UpdateRequiredExp`
  (params (newLevel :type Integer) (RequiredExp :type "Float (double-precision)"))
  ;[0 0.15 0.09537 0.5] 필요 Exp 설정 후 레벨 업 해야하는지 질의.
  (set `self.CurrentLevel` newLevel)
  (set `self.Exp` (- (`self.Exp`) (`self.RequiredExp`)))
  (bind _output_get (set `self.RequiredExp` RequiredExp))
  (`self.OnExpChanged` (`self.Exp`) _output_get)
  (if (>= (`self.Exp`) (`self.RequiredExp`))
    (`self.OnLevelUpRequested` (+ (`self.CurrentLevel`) 1))))
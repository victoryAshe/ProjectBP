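; Mana component that tracks current and maximum MP for its owner.
; Mana starts full on BeginPlay, and UpdateMaxMp sets a new maximum and refills to it without broadcasting.
; UseMana deducts a cost only when current mana strictly exceeds it and returns whether it succeeded.
; A successful spend fires the OnMpChanged dispatcher, whose parameters carry HealthPower names despite holding mana values.
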(event `self.ReceiveBeginPlay`
  ;[0.04024 0.15 0.01092 0.5] 최대 마나로 게임 시작
  (set `self.ManaPower` (`self.MaxManaPower`)))

(event `UpdateMaxMp`
  (params (MaxManaPower :type "Float (double-precision)"))
  ;[0 0.15 0.09537 0.5] 최대 Mana 설정.
  (bind _output_get (set `self.MaxManaPower` MaxManaPower))
  (set `self.ManaPower` _output_get))

(fn `UseMana`
  (params (ManaUse :type "Float (double-precision)"))
  (returns (bResult :type Boolean))
  ; 사용할 수 있는지 검사.
  (if (> (`self.ManaPower`) ManaUse)
    (bind _output_get (set `self.ManaPower` (- (`self.ManaPower`) ManaUse)))
    (`self.OnMpChanged` _output_get (`self.MaxManaPower`))
    (return true)
    (else
      (return false))))
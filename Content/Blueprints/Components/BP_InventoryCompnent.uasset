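; Inventory component that stores items in a fixed-size array of slot structs holding occupancy, item ID and count.
; OnInitialize sizes the array to MaxSlotCount, but its clearing loop returns after writing the first slot.
; AddItem stacks onto a matching ID without a cap, otherwise fills the first free slot, returning false when neither exists.
; RemoveItem is unfinished: it only stores the requested count, and its return is unconnected.
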(fn `AddItem`
  (params (ItemID :type Name) (AddCount :type Integer))
  (returns (bSuccess :type Boolean))
  ; 기존 Slot에 같은 Item 있는지 찾기.
  (for (_array_element _array_index) (`self.InventorySlots`)
    (bind (_boccupied _itemid _count) (break `/Game/Blueprints/Character/Data/FInventorySlotData` _array_element))
    (if (== _itemid (`local.ItemID`))
      (bind _structout (setmembers `/Game/Blueprints/Character/Data/FInventorySlotData` :`StructRef` _array_element :`Count` (+ _count (`local.AddCount`))))
      (`KismetArrayLibrary.Array_Set` (`self.InventorySlots`) _array_index _structout)
      (return true)))
  ; 빈 칸을 찾아 넣기.
  (for (_array_element_2 _array_index_2) (`self.InventorySlots`)
    (if (not (`.bOccupied_1_0796740C4C1C5A3B8504D99FC7BEFEC2` (break `/Game/Blueprints/Character/Data/FInventorySlotData` _array_element_2)))
      (bind _structout_2 (setmembers `/Game/Blueprints/Character/Data/FInventorySlotData` :`StructRef` _array_element_2 :`bOccupied` true :`ItemID` (`local.ItemID`) :`Count` (`local.AddCount`)))
      (`KismetArrayLibrary.Array_Set` (`self.InventorySlots`) _array_index_2 _structout_2)
      (return true)))
  (return false))

(fn `OnInitialize`
  (bind _maxslotcount (`self.MaxSlotCount`))
  (`KismetArrayLibrary.Array_Resize` (`self.InventorySlots`) _maxslotcount)
  (for _index (range _maxslotcount)
    (`KismetArrayLibrary.Array_Set` (`self.InventorySlots`) _index (make `/Game/Blueprints/Character/Data/FInventorySlotData` false))
    (return)))

(fn `RemoveItem`
  (params (ItemID :type Name) (RemoveCount :type Integer))
  (returns (RemovedCount :type Integer))
  (locals (RemainRemoveCount :type Integer))
  (set `local.RemainRemoveCount` RemoveCount))
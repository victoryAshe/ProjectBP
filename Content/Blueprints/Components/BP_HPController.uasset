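; BP_HPController is a health component that tracks current and maximum HP for its owner, starting at full health on BeginPlay.
; ReceiveDamage subtracts damage while HP is above zero, floors it at zero, and broadcasts OnHpChanged.
; On a lethal hit it fires OnDead before OnHpChanged, and later damage is ignored while HP stays at zero.
; UpdateMaxHp sets a new maximum and refills HP without broadcasting OnHpChanged.
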(event `self.ReceiveBeginPlay`
  ;[0.04024 0.15 0.01092 0.5] 최대 체력으로 게임 시작
  (set `self.HealthPower` (`self.MaxHealthPower`)))

(event `ReceiveDamage`
  (params (Damage :type "Float (double-precision)"))
  ;[0.15 0.0457 0 0.5] Process Damage + 체력 변경, 죽음 Event Binding
  (if (> (`self.HealthPower`) 0.0)
    (bind _output_get (set `self.HealthPower` (- (`self.HealthPower`) Damage)))
    (if (<= _output_get 0.0)
      (set `self.HealthPower` 0.0) ; 0미만의 값은 들어가지 않도록.
      (`self.OnDeadEvent`)
      (`self.OnHpChanged` (`self.HealthPower`) (`self.MaxHealthPower`)) ; 앞에서 처리해줄 수도 있는데 \n그게 더 까다로우니까 그냥 블록 아래에서 복붙
      (else
        (`self.OnHpChanged` (`self.HealthPower`) (`self.MaxHealthPower`)) ; 체력 값이 변경됐는데, 아직 살아있을 때.
      ))))

(event `UpdateMaxHp`
  (params (MaxHealthPower :type "Float (double-precision)"))
  ;[0 0.15 0.09537 0.5] 최대 체력 설정.
  (bind _output_get (set `self.MaxHealthPower` MaxHealthPower))
  (set `self.HealthPower` _output_get))
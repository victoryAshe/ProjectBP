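; Easy monster enemy that chases the player on sight, damages it through a notify-toggled attack collision, and reports its death to the game mode.
; A Tick-driven state machine (Locomotion, Chase, Attack, Dead) mirrors state to the AI Blackboard and sets walk speed from level-based MonsterData.
; AI perception starts chases, which end beyond a hardcoded distance.
; An HP controller drives the health bar and death, with timeline-animated hit flash and dissolve.
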(event `UpdateState`
  (params (NewState :type "/Game/Blueprints/Monster/EMonsterState Enum" :default "NewEnumerator0"))
  (bind _charactermovement (`self.CharacterMovement`))
  (bind (_currentleveldata_attack _currentleveldata_defence _currentleveldata_walkspeed _currentleveldata_chasespeed) (break `/Game/Blueprints/Monster/Data/BP_MonsterLevelData` (`/Game/Blueprints/Components/BP_MonsterData.GetCurrentLevelData` (`self.MonsterData`))))
  ;[0 0.09522 0.15 0.5] 몬스터 상태 변경 Event.
  (if (`|EnumInequality` (`self.State_BP`) "NewEnumerator3")
    (bind _output_get (set `self.State_BP` NewState))
    (`BlackboardComponent.SetValueAsEnum` (`AIController.Blackboard` (`AIBlueprintHelperLibrary.GetAIController` self)) (`self.StateKey`) _output_get)
    (switch `/Game/Blueprints/Monster/EMonsterState` (`self.State_BP`)
      (:`NewEnumerator0`
        (set `CharacterMovementComponent.MaxWalkSpeed` _currentleveldata_walkspeed _charactermovement))
      (:`NewEnumerator1`
        (set `CharacterMovementComponent.MaxWalkSpeed` _currentleveldata_chasespeed _charactermovement))
      (:`NewEnumerator2`
        (set `CharacterMovementComponent.MaxWalkSpeed` 0.0 _charactermovement :!label _label))
      (:`NewEnumerator3`
        (goto _label)))))

(event `ReceiveOnHpChanged`
  (params (HealthPower :type "Float (double-precision)") (MaxHealthPower :type "Float (double-precision)"))
  ;[0.04893 0.15 0.03589 0.5] Bind Events.
  ;;[0.1298 0 0.15 0.5] On Hp Change 이벤트 Binding.
  (bind _aswbp_hpbar (cast `/Game/UI/UI_fromLecture/WBP_HPBar` (`WidgetComponent.GetUserWidgetObject` (`self.HPBar`))))
  (`/Game/UI/UI_fromLecture/WBP_HPBar.UpdateHpPercent` _aswbp_hpbar (/ HealthPower MaxHealthPower)))

(event `self.ReceiveBeginPlay`
  (bind (_attack _defence _walkspeed _chasespeed _maxhp) (break `/Game/Blueprints/Monster/Data/BP_MonsterLevelData` (`/Game/Blueprints/Components/BP_MonsterData.GetCurrentLevelData` (`self.MonsterData`))))
  ;[0.04893 0.15 0.03589 0.5] Bind Events.
  (add `/Game/Blueprints/Components/BP_HPController.OnDeadEvent` (`self.BP_HPController`) (delegate `ReceiveOnDead`))
  ;; 시작할 때 AttackCollision Off.
  (`PrimitiveComponent.SetCollisionEnabled` (`self.AttackCollision`) "NoCollision")
  ;;[0.15 0.008393 0 0.5] Monster Level에 맞는 공격력/체력 설정.
  (`/Game/Blueprints/Components/BP_HPController.UpdateMaxHp` (`self.BP_HPController`) _maxhp)
  (set `self.Damage` _attack)
  ;;[0.1298 0 0.15 0.5] On Hp Change 이벤트 Binding.
  (add `/Game/Blueprints/Components/BP_HPController.OnHpChanged` (`self.BP_HPController`) (delegate `ReceiveOnHpChanged`)))

(event `ReceiveOnDead`
  (bind _mesh (`self.Mesh`))
  ;[0.04893 0.15 0.03589 0.5] Bind Events.
  ;;[0.1204 0 0.15 0.5] Monster의 죽음을 Game에 알림
  (bind _asbp_game_mode (cast `/Game/Blueprints/BP_GameMode` (`GameplayStatics.GetGameMode`)))
  (`/Game/Blueprints/BP_GameMode.MonsterKilled` _asbp_game_mode)
  (`self.UpdateState` "NewEnumerator3")
  (`PrimitiveComponent.SetCollisionEnabled` (`self.CapsuleComponent`) "NoCollision")
  (`KismetSystemLibrary.Delay` 1.0)
  ;;[0 0 0 0.5] 죽음 효과.
  (bind (_direction _dissolve _hitvalue) (`Timeline|DeathEffect` :!via `PlayFromStart`)
    (:`Update`
      (`MeshComponent.SetScalarParameterValueOnMaterials` _mesh "Dissolve" _dissolve)
      (`MeshComponent.SetScalarParameterValueOnMaterials` _mesh "HitValue" _hitvalue))
    (:`Finished`
      (`self.K2_DestroyActor`))))

(event `self.ReceiveAnyDamage`
  (params (Damage :type "Float (single-precision)") (DamageType :type "DamageType Object Reference") (InstigatedBy :type "Controller Object Reference") (DamageCauser :type "Actor Object Reference"))
  ;[0.15 0 0.001557 0.5] HP Controller가 Damage 받음
  (`self.TurnToTarget` DamageCauser)
  (`/Game/Blueprints/Components/BP_HPController.ReceiveDamage` (`self.BP_HPController`) Damage)
  ;[0 0.121 0.15 0.5] 피격효과 재생.
  (bind (_direction _hitvalue) (`Timeline|HitEffect` :!via `PlayFromStart`)
    (:`Update`
      (`MeshComponent.SetScalarParameterValueOnMaterials` (`self.Mesh`) "HitValue" _hitvalue))))

(event `self.AIPerception.OnTargetPerceptionUpdated`
  (params (Actor :type "Actor Object Reference") (Stimulus :type "AIStimulus Structure"))
  ;[0.06055 0 0.15 0.5] 시야 감지
  (if (`.bSuccessfullySensed` (break `AIStimulus` Stimulus))
    (if (`|EnumEquality` (`self.State_BP`) "NewEnumerator0")
      (if (`self.ActorHasTag` Actor "Player")
        (`BlackboardComponent.SetValueAsObject` (`AIController.Blackboard` (`AIBlueprintHelperLibrary.GetAIController` self)) (`self.TargetPlayerKey`) Actor)
        ;;[0 0.15 0.0319 0.502] Player가 죽었는지 확인
        (bind _asbp_character (cast `/Game/Blueprints/Character/BP_Character` Actor))
        (if (not (`|EnumEquality` (`/Game/Blueprints/Character/BP_Character.State_BP` _asbp_character) "NewEnumerator2"))
          (`self.UpdateState` "NewEnumerator1"))))))

(event `self.ReceiveTick`
  (params (DeltaSeconds :type "Float (single-precision)"))
  ;[0.04231 0.08866 0.1274] 간단한 FSM.
  (switch `/Game/Blueprints/Monster/EMonsterState` (`self.State_BP`)
    (:`NewEnumerator0`
      (`self.OnLocomotion`))
    (:`NewEnumerator1`
      (`self.OnChase`))
    (:`NewEnumerator2`
      (`self.OnAttack`))
    (:`NewEnumerator3`
      (`self.OnDead`))))

(event `OnAttackCheckStart`
  ;[0.15 0.04961 0.008295 0.5] 공격 판정 시작/종료: Attack Collision On/Off
  (`PrimitiveComponent.SetCollisionEnabled` (`self.AttackCollision`) "QueryOnly"))

(event `OnAttackCheckEnd`
  ;[0.15 0.04961 0.008295 0.5] 공격 판정 시작/종료: Attack Collision On/Off
  (`PrimitiveComponent.SetCollisionEnabled` (`self.AttackCollision`) "NoCollision"))

(event `self.AttackCollision.OnComponentBeginOverlap`
  (params (OverlappedComponent :type "PrimitiveComponent Object Reference") (OtherActor :type "Actor Object Reference") (OtherComp :type "PrimitiveComponent Object Reference") (OtherBodyIndex :type Integer) (bFromSweep :type Boolean) (SweepResult :type "HitResult Structure (by ref)"))
  ;[0.15 0 0.005816 0.5] Player에 Damage 전달.
  (`GameplayStatics.ApplyDamage` OtherActor (`self.Damage`) (`self.GetController`) self))

(fn `OnAttack`
  (bind _asbp_character (cast `/Game/Blueprints/Character/BP_Character` (`BlackboardComponent.GetValueAsObject` (`AIController.Blackboard` (`AIBlueprintHelperLibrary.GetAIController` self)) (`self.TargetPlayerKey`))))
  ;[0 0.15 0.0319 0.502] Player가 죽었는지 확인
  (if (`|EnumEquality` (`/Game/Blueprints/Character/BP_Character.State_BP` _asbp_character) "NewEnumerator2")
    (`self.UpdateState` "NewEnumerator0") ; Locomotion으로 돌아가기.
  ))

(fn `OnChase`
  (bind _asactor (cast `Actor` (`BlackboardComponent.GetValueAsObject` (`AIController.Blackboard` (`AIBlueprintHelperLibrary.GetAIController` self)) (`self.TargetPlayerKey`))))
  (if (> (`KismetMathLibrary.Vector_Distance` (`self.K2_GetActorLocation` _asactor) (`self.K2_GetActorLocation`)) 400.0)
    (`self.UpdateState` "NewEnumerator0") ; Locomotion으로 상태를 바꿔줘야 함\n=> Monster가 Roaming하도록.
  ))

(fn `OnDead`)

(fn `OnLocomotion`)

(fn `TurnToTarget`
  (params (TargetActor :type "Actor Object Reference"))
  (bind (_returnvalue_roll _returnvalue_pitch _returnvalue_yaw) (`KismetMathLibrary.BreakRotator` (`KismetMathLibrary.MakeRotFromX` (- (`self.K2_GetActorLocation` TargetActor) (`self.K2_GetActorLocation`)))))
  (switch `/Game/Blueprints/Monster/EMonsterState` (`self.State_BP`)
    (:`NewEnumerator0`
      (`self.K2_SetActorRotation` (`KismetMathLibrary.MakeRotator` 0.0 0.0 _returnvalue_yaw)))))

(fn `UserConstructionScript`
  (`PrimitiveComponent.SetCastShadow` (`self.HPBar`) false))
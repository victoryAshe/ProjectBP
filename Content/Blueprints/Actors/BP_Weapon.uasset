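; BP_Weapon is a collectible melee weapon actor that damages what it hits during attack windows.
; Overlapping its Sphere passes the weapon to BP_Character through OnWeaponCollected, then disables the pickup collision.
; AttackCollision starts disabled and is toggled to query-only by the OnAttackCheckBegin and OnAttackCheckEnd events.
; Its overlaps call ApplyDamage with the Damage variable, crediting player controller 0 as instigator.
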(event `self.ReceiveBeginPlay`
  ; 공격 Collision 끄기.
  (`PrimitiveComponent.SetCollisionEnabled` (`self.AttackCollision`) "NoCollision"))

(event `self.Sphere.OnComponentBeginOverlap`
  (params (OverlappedComponent :type "PrimitiveComponent Object Reference") (OtherActor :type "Actor Object Reference") (OtherComp :type "PrimitiveComponent Object Reference") (OtherBodyIndex :type Integer) (bFromSweep :type Boolean) (SweepResult :type "HitResult Structure (by ref)"))
  ;[1 0.6403 0.054 0.5] 무기 습득 처리.
  (bind _asbp_character (cast `/Game/Blueprints/Character/BP_Character` OtherActor))
  (`/Game/Blueprints/Character/BP_Character.OnWeaponCollected` _asbp_character self)
  (`PrimitiveComponent.SetCollisionEnabled` (`self.Sphere`) "NoCollision"))

(event `OnAttackCheckBegin`
  ;[0 0.162 0.926 0.5] 공격 판정 시작.
  (`PrimitiveComponent.SetCollisionEnabled` (`self.AttackCollision`) "QueryOnly"))

(event `self.AttackCollision.OnComponentBeginOverlap`
  (params (OverlappedComponent :type "PrimitiveComponent Object Reference") (OtherActor :type "Actor Object Reference") (OtherComp :type "PrimitiveComponent Object Reference") (OtherBodyIndex :type Integer) (bFromSweep :type Boolean) (SweepResult :type "HitResult Structure (by ref)"))
  ;[0.574 0 0 0.5] Damage 전달.
  (`GameplayStatics.ApplyDamage` OtherActor (`self.Damage`) (`GameplayStatics.GetPlayerController` 0) self))

(event `OnAttackCheckEnd`
  ;[0.602 0 0 0.5] 공격 판정 종료.
  (`PrimitiveComponent.SetCollisionEnabled` (`self.AttackCollision`) "NoCollision"))

(fn `UserConstructionScript`)
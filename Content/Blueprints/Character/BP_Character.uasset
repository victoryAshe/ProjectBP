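; Player character Blueprint handling weapon combo attacks, health, death and camera zoom.
; Holding attack with a collected, socket-attached weapon starts a montage and queues the next combo by current section.
; Attack-check events reach the weapon through dispatchers bound on pickup.
; Damage feeds BPHPController, which drives the HP bar and death state, and plays a material hit flash; Tick eases spring-arm length, then pitch, while zoom flags are set.
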(event `self.ReceiveBeginPlay`
  ;[0.02315 0.05613 0.05286] 시작 시: 죽음 Event에 Binding.
  (add `/Game/Blueprints/Components/BP_HPController.OnDeadEvent` (`self.BP_HPController`) (delegate `Receive OnDeadEvent`))
  (add `/Game/Blueprints/Components/BP_HPController.OnHpChanged` (`self.BP_HPController`) (delegate `ReceiveOnHpChanged`)))

(event `ReceiveOnHpChanged`
  (params (HealthPower :type "Float (double-precision)") (MaxHealthPower :type "Float (double-precision)"))
  ;[0.02315 0.05613 0.05286] 시작 시: 죽음 Event에 Binding.
  (bind _aswbp_hpbar (cast `/Game/UI/WBP_HPBar` (`WidgetComponent.GetUserWidgetObject` (`self.HPBar`))))
  (`/Game/UI/WBP_HPBar.UpdateHpPercent` _aswbp_hpbar (/ HealthPower MaxHealthPower)))

(event `Receive OnDeadEvent`
  ;[0.02315 0.05613 0.05286] 시작 시: 죽음 Event에 Binding.
  (`PrimitiveComponent.SetCollisionEnabled` (`self.CapsuleComponent`) "NoCollision") ; Collision 비활성화
  (set `self.State_BP` "NewEnumerator2"))

(event `self.ReceiveTick`
  (params (DeltaSeconds :type "Float (single-precision)"))
  (bind _springarm (`self.SpringArm`))
  (bind _springarm_2 (`self.SpringArm`))
  (bind (_returnvalue_roll _returnvalue_pitch _returnvalue_yaw) (`KismetMathLibrary.BreakRotator` (`KismetMathLibrary.RInterpTo` (`SceneComponent.RelativeRotation` (`self.SpringArm`)) (`self.ZoomInRotator`) DeltaSeconds (`self.ArmRotationSpeed`))))
  (bind (_returnvalue_roll_2 _returnvalue_pitch_2 _returnvalue_yaw_2) (`KismetMathLibrary.BreakRotator` (`KismetMathLibrary.RInterpTo` (`SceneComponent.RelativeRotation` (`self.SpringArm`)) (`self.ZoomOutRotator`) DeltaSeconds (`self.ArmRotationSpeed`))))
  (bind _returnvalue (`KismetMathLibrary.FClamp` _returnvalue_pitch -50.0 -15.0))
  (bind _returnvalue_2 (`KismetMathLibrary.FClamp` _returnvalue_pitch_2 -50.0 -15.0))
  ; 매 Tick마다 카메라 길이 검사 및 변경
  (if (`self.bZoomOut`)
    (if (< (`SpringArmComponent.TargetArmLength` (`self.SpringArm`)) (`self.ZoomOutArmLength`))
      (set `SpringArmComponent.TargetArmLength` (`KismetMathLibrary.FClamp` (+ (`SpringArmComponent.TargetArmLength` _springarm) (`self.ArmLengthSpeed`)) (`self.ZoomInArmLength`) (`self.ZoomOutArmLength`)) _springarm)
      (else
        (`SceneComponent.K2_SetRelativeRotation` (`self.SpringArm`) (`KismetMathLibrary.MakeRotator` _returnvalue_roll_2 _returnvalue_2 _returnvalue_yaw_2) false false)
        (if (== _returnvalue_2 -50.0)
          (set `self.bZoomOut` false))))
    (elif (`self.bZoomIn`)
      (if (> (`SpringArmComponent.TargetArmLength` (`self.SpringArm`)) (`self.ZoomInArmLength`))
        (set `SpringArmComponent.TargetArmLength` (`KismetMathLibrary.FClamp` (- (`SpringArmComponent.TargetArmLength` _springarm_2) (`self.ArmLengthSpeed`)) (`self.ZoomInArmLength`) (`self.ZoomOutArmLength`)) _springarm_2)
        (else
          (`SceneComponent.K2_SetRelativeRotation` (`self.SpringArm`) (`KismetMathLibrary.MakeRotator` _returnvalue_roll _returnvalue _returnvalue_yaw) false false)
          (if (== _returnvalue -15.0)
            (set `self.bZoomIn` false)))))))

(event `OnAttackCheckBegin`
  ;[0.15 0 0 0.5] 공격 판정 시작
  (`self.AttackCheckBeginEvent`))

(event `OnAttackCheckEnd`
  ;[0.02247 0.15 0.006907 0.5] 공격판정 종료.
  (`self.AttackCheckEndEvent`))

(event `EnhancedInput|/Game/Blueprints/Input/Actions/IA_Attack_RightClick`
  (params (ActionValue :type Boolean) (ElapsedSeconds :type "Float (double-precision)") (TriggeredSeconds :type "Float (double-precision)") (InputAction :type "InputAction Object Reference" :default "/Game/Blueprints/Input/Actions/IA_Attack_RightClick.IA_Attack_RightClick"))
  ;[0.15 0 0.006727 0.5] 공격.
  (:`Triggered`
    (if (`self.bAttackHeld`)
      (if (`self.bHasWeapon`)
        ;; 일반 상태인지 확인
        (switch `/Game/Blueprints/Character/EPlayerState` (`self.State_BP`)
          (:`NewEnumerator0`
            (set `self.State_BP` "NewEnumerator1")
            (`self.PlayAnimMontage` "/Game/Blueprints/Character/AM_Attack.AM_Attack"))
          (:`NewEnumerator1`
            (if (`self.bAttackHeld`)
              (switch `name` (`AnimInstance.Montage_GetCurrentSection` (`SkeletalMeshComponent.GetAnimInstance` (`self.Mesh`)) "/Game/Blueprints/Character/AM_Attack.AM_Attack")
                (:`Attack1`
                  (set `self.NextCombo` "Attack2"))
                (:`Attack2`
                  (set `self.NextCombo` "Attack3"))
                (:`Attack3`
                  (set `self.NextCombo` "Attack4")))))))))
  (:`Started`
    (set `self.bAttackHeld` true))
  (:`Canceled`
    (set `self.bAttackHeld` false :!label _label))
  (:`Completed`
    (goto _label)))

(event `AttackEnd`
  ;[0.15 0 0.006727 0.5] 공격.
  (set `self.State_BP` "NewEnumerator0"))

(event `OnWeaponCollected`
  (params (WeaponActor :type "/Game/Blueprints/Actors/BP_Weapon Object Reference"))
  ;[0 0.798 0.04515 0.5] 무기 습득 처리.
  (`self.SetOwner` WeaponActor self)
  (`self.K2_AttachToComponent` WeaponActor (`self.Mesh`) "WeaponPosition" "SnapToTarget" "SnapToTarget" "SnapToTarget" true)
  (set `self.WeaponActor` WeaponActor)
  (set `self.bHasWeapon` true)
  ;[0.759 0 0 0.5] 공격 판정 시작 Event 함수 등록(Subscription) => Observer Pattern.
  (add `self.AttackCheckBeginEvent` (delegate `RaiseAttackCheckBegin`))
  ;[0 0.36 0.1518 0.5] 공격 판정 종료 Event에 함수 등록(Subscription)
  (add `self.AttackCheckEndEvent` (delegate `RaiseAttackCheckEnd`)))

(event `RaiseAttackCheckBegin`
  ;[0.759 0 0 0.5] 공격 판정 시작 Event 함수 등록(Subscription) => Observer Pattern.
  (`/Engine/EditorBlueprintResources/StandardMacros.IsValid` (`self.WeaponActor`)
    (:`Is Valid`
      (`/Game/Blueprints/Actors/BP_Weapon.OnAttackCheckBegin` (`self.WeaponActor`)))))

(event `RaiseAttackCheckEnd`
  ;[0 0.36 0.1518 0.5] 공격 판정 종료 Event에 함수 등록(Subscription)
  (`/Engine/EditorBlueprintResources/StandardMacros.IsValid` (`self.WeaponActor`)
    (:`Is Valid`
      (`/Game/Blueprints/Actors/BP_Weapon.OnAttackCheckEnd` (`self.WeaponActor`)))))

(event `self.ReceiveAnyDamage`
  (params (Damage :type "Float (single-precision)") (DamageType :type "DamageType Object Reference") (InstigatedBy :type "Controller Object Reference") (DamageCauser :type "Actor Object Reference"))
  ;[0.15 0 0.123 0.5] 체력 관리 Component에 Damage 전달.
  (`/Game/Blueprints/Components/BP_HPController.ReceiveDamage` (`self.BP_HPController`) Damage)
  (bind (_direction _hitvalue) (`Timeline|HitEffect` :!via `PlayFromStart`)
    (:`Update`
      (`MeshComponent.SetScalarParameterValueOnMaterials` (`self.Mesh`) "HitValue" _hitvalue))))

(fn `UserConstructionScript`
  (`PrimitiveComponent.SetCastShadow` (`self.HPBar`) false)
  (`parent.UserConstructionScript`))
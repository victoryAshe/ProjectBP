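; BP_GameMode is the dungeon game mode, tracking kill progress and relaying game start, game over, stage clear and player HP changes.
; Its events re-broadcast through dispatchers, with each monster kill incrementing the count and firing stage clear when it equals the target.
; LoadLevel streams in the second dungeon sublevel without blocking, while RestartGame opens the out-of-dungeon level.
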(event `LoadLevel`
  ;[0.004326 0.09918 0.15 0.5] 다음 Section 로드
  (`GameplayStatics.LoadStreamLevelBySoftObjectPtr` "/Game/Levels/Level_Dungeon_SubLevel2.Level_Dungeon_SubLevel2" true))

(event `GameStart`
  ;[0.15 0.1425 0.04699 0.5] 게임 시작 Event.
  (`self.OnGameStart`)
  (`self.OnKillCountUpdated` (`self.CurrentKills`) (`self.TargetKills`)))

(event `MonsterKilled`
  (bind _result (`/Engine/EditorBlueprintResources/StandardMacros.IncrementInt` (`self.CurrentKills`))
    (:`  `
      (`self.OnKillCountUpdated` _result (`self.TargetKills`))
      ; Stage Clear 조건 확인 및 Event 발행
      (if (== (`self.CurrentKills`) (`self.TargetKills`))
        (`self.OnStageClear`)))))

(event `PlayerDied`
  ; Game Over
  (`self.OnGameOver`))

(event `RestartGame`
  ; 게임 재시작
  (`GameplayStatics.OpenLevelBySoftObjectPtr` "/Game/Levels/Level_OutOfDungeon.Level_OutOfDungeon"))

(event `PlayerHpChanged`
  (params (healthPower :type "Float (double-precision)") (maxHealthPower :type "Float (double-precision)"))
  ; Screen Player HP UI => Change Event
  (`self.OnPlayerHpChanged` healthPower maxHealthPower))

(fn `UserConstructionScript`)